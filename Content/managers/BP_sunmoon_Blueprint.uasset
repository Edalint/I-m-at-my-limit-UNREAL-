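; Sun manager Blueprint for a day-night cycle that tracks an hour of day and is built to pitch the Sun accordingly.
; Tick advances Currenthour, scaled by Dayinrealminutes and wrapped at 24 with modulo.
; The Branch condition is fixed true with the hour comparison unconnected, so it subtracts 24 every tick and never reaches the Sun rotation on the false path.
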(event EventTick
  (params (DeltaSeconds :type Float%20%28single-precision%29))
  (bind _output_get (Variables|Default|Setcurrenthour (Math|Float|%(Float) (+ (* DeltaSeconds (/ 24.0 (* (Variables|Default|Getdayinrealminutes) 6e+01))) (Variables|Default|Getcurrenthour)) 24.0))) ; EL VALOR A CAMBIAR
  (Utilities|FlowControl|Sequence
    (:then_0
      (if true ; IF
        (Variables|Default|Setcurrenthour (- (Variables|Default|Getcurrenthour) 24.0))
        (else
          (Transformation|SetWorldRotation (Variables|Default|GetSun) (Math|Rotator|MakeRotator 0.0 (- (* (/ (Variables|Default|Getcurrenthour) 24.0) 3.6e+02) 2.7e+02) 0.0) false false))))))

(fn ConstructionScript)