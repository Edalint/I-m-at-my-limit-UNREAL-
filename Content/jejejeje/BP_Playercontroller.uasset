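; Player controller that drives BP_Player's third-person camera and movement through Enhanced Input.
; On BeginPlay it sets game-only input, caches the pawn and its camera, and adds the gameplay mapping context.
; Camera input rotates the spring arm directly with scaled yaw and clamped pitch.
; Movement input moves the pawn along the camera's forward and right vectors and snaps the mesh's yaw to that direction.
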(event Input|EnhancedActionEvents|EnhancedInputActionIA_Camera
  (params (ActionValue :type Vector%202D%20Structure) (ElapsedSeconds :type Float%20%28double-precision%29) (TriggeredSeconds :type Float%20%28double-precision%29) (InputAction :type Input%20Action%20Object%20Reference :default "/Game/managers/inputs/IA_Camera.IA_Camera"))
  (CallFunction|MoveCamera ActionValue))

(event Input|EnhancedActionEvents|EnhancedInputActionIA_Movement
  (params (ActionValue :type Vector%202D%20Structure) (ElapsedSeconds :type Float%20%28double-precision%29) (TriggeredSeconds :type Float%20%28double-precision%29) (InputAction :type Input%20Action%20Object%20Reference :default "/Game/managers/inputs/IA_Movement.IA_Movement"))
  (CallFunction|MoveCharacter ActionValue))

(event EventBeginPlay
  (CallFunction|InitController))

(event EventTick
  (params (DeltaSeconds :type Float%20%28single-precision%29)))

(fn ConstructionScript)

(fn InitController
  (Input|SetInputModeGameOnly self false)
  (bind _asbp_player (Utilities|Casting|CastToBP_Player (Pawn|GetControlledPawn)))
  (bind _output_get (Variables|References|SetplayerRef _asbp_player))
  (Variables|References|SetplayerCam (Variables|/Game/jejejeje/BP_Player.BP_Player_C|GetCamera _output_get))
  (Input|AddMappingContext (PlayerController|LocalPlayerSubsystems|GetEnhancedInputLocalPlayerSubsystem) "/Game/managers/inputs/IM_Gameplay.IM_Gameplay" 0 "(bIgnoreAllPressedKeysUntilRelease=True,bForceImmediately=False,bNotifyUserSettings=False)"))

(fn MoveCamera
  (params (InVec :type Vector%202D%20Structure))
  (bind (_x _y) (Math|Vector2D|BreakVector2D InVec))
  (bind _playerref (Variables|References|GetplayerRef)
    (:then
      (Transformation|SetRelativeRotation (Variables|/Game/jejejeje/BP_Player.BP_Player_C|GetSpringArm _playerref) (Math|Rotator|MakeRotator 0.0 (Math|Float|Clamp(Float) (+ (.Pitch (Math|Rotator|BreakRotator (Variables|/Script/Engine.SceneComponent|GetRelativeRotation (Variables|/Game/jejejeje/BP_Player.BP_Player_C|GetSpringArm _playerref)))) (* _y (Variables|Default|GetCamSpeedY))) (Variables|Default|GetMinAngleY) (Variables|Default|GetMaxAngleY)) (+ (.Yaw (Math|Rotator|BreakRotator (Variables|/Script/Engine.SceneComponent|GetRelativeRotation (Variables|/Game/jejejeje/BP_Player.BP_Player_C|GetSpringArm _playerref)))) (* _x (Variables|Default|GetCamSpeedX)))) false false))
    (:else)))

(fn MoveCharacter
  (params (InVec :type Vector%202D%20Structure))
  (bind (_x _y) (Math|Vector2D|BreakVector2D InVec))
  (bind _playerref (Variables|References|GetplayerRef)
    (:then
      (bind _playercam (Variables|References|GetplayerCam)
        (:then
          (Pawn|Input|AddMovementInput _playerref (+ (* _x (Math|Vector|GetForwardVector _playercam)) (* _y (Math|Vector|GetRightVector _playercam))) 1.0 false)
          (Transformation|SetWorldRotation (Variables|/Script/Engine.Character|GetMesh _playerref) (Math|Rotator|MakeRotator 0.0 0.0 (.yaw (Math|Rotator|MakeRotfromX (Math|Vector|Normalize (+ (* _x (Math|Vector|GetForwardVector _playercam)) (* _y (Math|Vector|GetRightVector _playercam))))))) false false))
        (:else)))
    (:else)))